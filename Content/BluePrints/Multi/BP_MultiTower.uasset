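; BP_MultiTower is a tower that picks a BP_MultiMonster in its attack range and turns its cannon toward it.
; AttackRange overlaps maintain a target list, and a random entry is chosen when there is no current target or the current one leaves.
; Gated, self-recalling Delay loops smoothly rotate CannonMesh toward the target, or back to zero rotation when none remains.
; The graph handles targeting and aiming only, with no firing logic.
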(event `ContinueAim`
  (bind _cannonmesh (`self.CannonMesh`))
  ;[1 1 1] Aim Monster
  (`/Engine/EditorBlueprintResources/StandardMacros.IsValid` (`self.CurrentTarget`)
    (:`Is Valid`
      (`/Engine/EditorBlueprintResources/StandardMacros.Gate` true :!label _label
        (:`Exit`
          (`/Engine/EditorBlueprintResources/StandardMacros.IsValid` (`self.CurrentTarget`)
            (:`Is Valid`
              ;;[1 1 1] 몬스터 위치값 가져옴
              (set `self.MonsterTargetLoc` (`self.K2_GetActorLocation` (`self.CurrentTarget`)))
              (`SceneComponent.K2_SetRelativeRotation` _cannonmesh (`KismetMathLibrary.RInterpTo` (`SceneComponent.RelativeRotation` _cannonmesh) (`KismetMathLibrary.FindLookAtRotation` (- (`self.K2_GetActorLocation` (`self.CurrentTarget`)) (`self.MonsterTargetLoc`)) (`KismetMathLibrary.InverseTransformDirection` (`self.GetTransform`) (- (`self.MonsterTargetLoc`) (`SceneComponent.K2_GetComponentLocation` (`self.CannonMesh`))))) (`GameplayStatics.GetWorldDeltaSeconds`) 5.0) false false)
              (`KismetSystemLibrary.Delay` (`GameplayStatics.GetWorldDeltaSeconds`))
              (`self.ContinueAim`))
            (:`Is Not Valid`
              (`self.CancelAim`)
              (`self.BeginReset`))))))
    (:`Is Not Valid`
      (`self.CancelAim`)
      (`self.BeginReset`))))

(event `BeginAim`
  ;[1 1 1] Aim Monster
  (`|ExecutionSequence`
    (:`then_0`
      (goto _label :!via `Open`))
    (:`then_1`
      (goto _label))))

(event `CancelAim`
  ;[1 1 1] Aim Monster
  (goto _label :!via `Close`))

(event `ContinueRest`
  (bind _returnvalue (`KismetMathLibrary.RInterpTo` (`SceneComponent.RelativeRotation` (`self.CannonMesh`)) (struct) (`GameplayStatics.GetWorldDeltaSeconds`) 5.0))
  ;[1 1 1] Aim Reset
  (`/Engine/EditorBlueprintResources/StandardMacros.Gate` true :!label _label_2
    (:`Exit`
      (`/Engine/EditorBlueprintResources/StandardMacros.IsValid` (`self.CurrentTarget`)
        (:`Is Valid`
          (`self.CancelRest` :!label _label_3))
        (:`Is Not Valid`
          (if (== _returnvalue (struct))
            (goto _label_3)
            (else
              (`SceneComponent.K2_SetRelativeRotation` (`self.CannonMesh`) _returnvalue false false)
              (`KismetSystemLibrary.Delay` (`GameplayStatics.GetWorldDeltaSeconds`))
              (`self.ContinueRest`))))))))

(event `BeginReset`
  ;[1 1 1] Aim Reset
  (`|ExecutionSequence`
    (:`then_0`
      (goto _label_2 :!via `Open`))
    (:`then_1`
      (goto _label_2))))

(event `SelectTarget`
  (bind _multimonstertarget (`self.MultiMonsterTarget`))
  ;[1 1 1] Select Target
  (if (`KismetArrayLibrary.Array_IsValidIndex` _multimonstertarget)
    (set `self.CurrentTarget` (`|GetArrayItem` _multimonstertarget (`KismetMathLibrary.RandomIntegerInRange` 0 (`KismetArrayLibrary.Array_LastIndex` _multimonstertarget))))
    ;;[1 1 1] 공격범위 체크
    (`self.BeginAim`)
    (else
      (`self.BeginReset`))))

(event `CancelRest`
  ;[1 1 1] Aim Reset
  (goto _label_2 :!via `Close`))

(event `self.AttackRange.OnComponentBeginOverlap`
  (params (OverlappedComponent :type "PrimitiveComponent Object Reference") (OtherActor :type "Actor Object Reference") (OtherComp :type "PrimitiveComponent Object Reference") (OtherBodyIndex :type Integer) (bFromSweep :type Boolean) (SweepResult :type "HitResult Structure (by ref)"))
  ;[1 1 1] Overlap탐지
  (bind _asbp_multi_monster (cast `/Game/BluePrints/Multi/BP_MultiMonster` OtherActor))
  (`KismetArrayLibrary.Array_Add` (`self.MultiMonsterTarget`) _asbp_multi_monster)
  (`/Engine/EditorBlueprintResources/StandardMacros.IsValid` (`self.CurrentTarget`)
    (:`Is Not Valid`
      (`self.SelectTarget`))))

(event `self.AttackRange.OnComponentEndOverlap`
  (params (OverlappedComponent :type "PrimitiveComponent Object Reference") (OtherActor :type "Actor Object Reference") (OtherComp :type "PrimitiveComponent Object Reference") (OtherBodyIndex :type Integer))
  ;[1 1 1] Overlap탐지
  (bind _asbp_multi_monster (cast `/Game/BluePrints/Multi/BP_MultiMonster` OtherActor))
  (if (`KismetArrayLibrary.Array_Contains` (`self.MultiMonsterTarget`) _asbp_multi_monster)
    (`KismetArrayLibrary.Array_RemoveItem` (`self.MultiMonsterTarget`) _asbp_multi_monster)
    (if (== _asbp_multi_monster (`self.CurrentTarget`))
      (set `self.CurrentTarget` null)
      (`self.SelectTarget`))))

(fn `UserConstructionScript`)