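; BP_Tower is a tower actor whose cannon tracks a monster, taking the first BP_Monster found at BeginPlay as its only target.
; Each Tick checks cannon-to-monster distance, aiming within a fixed range and otherwise easing back to zero rotation.
; Aiming converts the target direction into actor-local space and smooths the cannon's relative rotation with RInterpTo.
; A Shoot function spawns a projectile at the Arrow's transform, but nothing in this Blueprint calls it.
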(event `self.ReceiveBeginPlay`
  ;[1 1 1] Get Targets
  (bind _outactors (`GameplayStatics.GetAllActorsOfClass` "/Game/BluePrints/BP_Monster.BP_Monster_C"))
  (set `self.MonsterTarget` (`|GetArrayItem` _outactors)))

(event `self.ReceiveTick`
  (params (DeltaSeconds :type "Float (single-precision)"))
  ;[1 1 1] 타겟과 캐논 사이 거리로 조준/비조준
  ;;[1 1 1] 몬스터 위치값 가져옴
  (bind _output_get (set `self.MonsterTargetLoc` (`self.K2_GetActorLocation` (`self.MonsterTarget`))))
  ;;[1 1 1] 타워랑 몬스터 사이 간격 체크
  (if (<= (`KismetMathLibrary.VSize` (- _output_get (`SceneComponent.K2_GetComponentLocation` (`self.CannonMesh`)))) 500.0)
    ;[1 1 1] 공격범위 체크
    (`self.AimMonster`)
    (else
      (`self.ResetAim`))))

(event `AimMonster`
  (bind _cannonmesh (`self.CannonMesh`))
  ;[1 1 1] Aim Monster
  (`SceneComponent.K2_SetRelativeRotation` _cannonmesh (`KismetMathLibrary.RInterpTo` (`SceneComponent.RelativeRotation` _cannonmesh) (`KismetMathLibrary.FindLookAtRotation` (- (`self.K2_GetActorLocation` (`self.MonsterTarget`)) (`self.MonsterTargetLoc`)) (`KismetMathLibrary.InverseTransformDirection` (`self.GetTransform`) (- (`self.MonsterTargetLoc`) (`SceneComponent.K2_GetComponentLocation` (`self.CannonMesh`))))) (`GameplayStatics.GetWorldDeltaSeconds`) 5.0) false false))

(event `ResetAim`
  (bind _cannonmesh (`self.CannonMesh`))
  ;[1 1 1] Aim Reset
  (`SceneComponent.K2_SetRelativeRotation` _cannonmesh (`KismetMathLibrary.RInterpTo` (`SceneComponent.RelativeRotation` _cannonmesh) (struct) (`GameplayStatics.GetWorldDeltaSeconds`) 5.0) false false))

(fn `Shoot`
  (`|SpawnActorFromClass` (`self.ProjectileSpawn`) (`SceneComponent.K2_GetComponentToWorld` (`self.Arrow`)) "Undefined" "OverrideRootScale" null null))

(fn `UserConstructionScript`)