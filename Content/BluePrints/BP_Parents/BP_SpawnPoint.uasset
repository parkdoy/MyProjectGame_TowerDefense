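; Monster spawn point that releases escalating waves of BP_MultiMonster_Parent AI at its own location on a repeating countdown.
; Tick uses a Delay to count down about once a second, then calls SpawnMonster and resets the timer.
; Each spawn receives the current health and speed, while the batch size grows per wave until a Calc-based limit resets it.
; Every fifth loop raises the wave level, monster health and speed.
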(event `self.ReceiveBeginPlay`
  (`self.EnableInput` (`GameplayStatics.GetPlayerController` 0)))

(event `self.ReceiveTick`
  (params (DeltaSeconds :type "Float (single-precision)"))
  (`KismetSystemLibrary.Delay` 1.0)
  ;[1 1 1] 카운트다운
  (bind _result (`/Engine/EditorBlueprintResources/StandardMacros.DecrementInt` (`self.TimeSec`))
    (:`  `
      (bind _output_get (set `self.TimeSec` _result))
      (`KismetSystemLibrary.PrintString` (`KismetStringLibrary.Conv_IntToString` _output_get) false false)
      (if (< _output_get 0)
        (set `self.TimeSec` 3)
        (`self.SpawnMonster`)
        (bind _result_2 (`/Engine/EditorBlueprintResources/StandardMacros.IncrementFloat` (`self.LoopCount`))
          (:`  `
            (if (== (mod _result_2 5.0) 0.0)
              (`/Engine/EditorBlueprintResources/StandardMacros.IncrementFloat` (`self.MonsterHealth`)
                (:`  `
                  (set `self.MonsterSpeed` (+ (`self.MonsterSpeed`) 10.0)))))))))))

(event `SpawnMonster`
  (bind _calc (`self.Calc`))
  ;[1 1 1] 단계가 올라가면 증가하도록
  (`self.Wave`)
  (set `self.WaveRound` (+ (`KismetMathLibrary.FTrunc` (mod (`self.LoopCount`) _calc)) 1))
  (for _ (range (`self.SpawnCount`))
    (bind _returnvalue (`AIBlueprintHelperLibrary.SpawnAIFromClass` "/Game/BluePrints/BP_Parents/BP_MultiMonster_Parent.BP_MultiMonster_Parent_C" null (`self.K2_GetActorLocation`) (`self.K2_GetActorRotation`) true null))
    (`/Engine/EditorBlueprintResources/StandardMacros.IsValid` _returnvalue
      (:`Is Valid`
        (`Pawn.SpawnDefaultController` _returnvalue)
        (bind _asbp_multi_monster_parent (cast `/Game/BluePrints/BP_Parents/BP_MultiMonster_Parent` _returnvalue))
        (bind _output_get (set `/Game/BluePrints/BP_Parents/BP_MultiMonster_Parent.Health` (`self.MonsterHealth`) _asbp_multi_monster_parent))
        (bind _output_get_2 (set `/Game/BluePrints/BP_Parents/BP_MultiMonster_Parent.MovingSpeed` (`self.MonsterSpeed`) _asbp_multi_monster_parent))
        (`KismetSystemLibrary.PrintString` (`KismetStringLibrary.Concat_StrStr` "Speed :  " (`KismetStringLibrary.Conv_DoubleToString` _output_get_2) "Health : " (`KismetStringLibrary.Conv_DoubleToString` _output_get))))))
  (bind _output_get_3 (set `self.SpawnCount` (+ (`self.SpawnCount`) 1)))
  (if (> _output_get_3 (`KismetMathLibrary.FTrunc` (- _calc 1.0)))
    (set `self.SpawnCount` 0)
    (set `self.MonsterIncrease` 0)))

(event `Wave`
  (if (== (mod (`self.LoopCount`) 5.0) 0.0)
    (`/Engine/EditorBlueprintResources/StandardMacros.IncrementInt` (`self.WaveLevel`))))

(fn `NewFunction_0`
  (returns (Spawn :type Boolean))
  (bind _result (`/Engine/EditorBlueprintResources/StandardMacros.DecrementInt` (`self.TimeSec`))
    (:`  `
      (bind _output_get (set `self.TimeSec` _result))
      (`KismetSystemLibrary.PrintString` (`KismetStringLibrary.Conv_IntToString` _output_get))
      (if (< _output_get 0)
        (set `self.TimeSec` 20)
        (return false)
        (else
          (return true))))))

(fn `UserConstructionScript`)