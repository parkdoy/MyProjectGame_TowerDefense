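; Parent Blueprint for a homing projectile that damages multi-monsters (BP_MultiMonster_Parent).
; On BeginPlay it scans all such monsters, keeps the last one found within ProjectileRange, and sets a SceneComponent of that monster as the ProjectileMovement homing target.
; Tick destroys it once its straight-line distance from spawn reaches that range.
; Overlapping a monster applies damage once, destroys the projectile and spawns a small explosion.
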(event `self.ReceiveBeginPlay`
  (bind _projectilemovement (`self.ProjectileMovement`))
  (set `self.StartLoc` (`self.K2_GetActorLocation`))
  (bind _outactors (`GameplayStatics.GetAllActorsOfClass` "/Game/BluePrints/BP_Parents/BP_MultiMonster_Parent.BP_MultiMonster_Parent_C"))
  (for _array_element _outactors
    (if (< (`KismetMathLibrary.VSize` (- (`self.K2_GetActorLocation` _array_element) (`self.K2_GetActorLocation`))) (`self.ProjectileRange`))
      (set `self.HomingTarget` _array_element)))
  (bind _output_get (set `self.SetTargeting` (`self.GetComponentByClass` (`self.HomingTarget`) "/Script/Engine.SceneComponent")))
  (set `ProjectileMovementComponent.HomingTargetComponent` _output_get _projectilemovement)
  (set `ProjectileMovementComponent.bIsHomingProjectile` true _projectilemovement))

(event `self.ReceiveTick`
  (params (DeltaSeconds :type "Float (single-precision)"))
  ;[1 1 1] 유효사거리 범위 넘어가면 사라지도록
  (if (>= (`KismetMathLibrary.VSize` (- (`self.StartLoc`) (`self.K2_GetActorLocation`))) (`self.ProjectileRange`))
    (`/Engine/EditorBlueprintResources/StandardMacros.DoOnce` false
      (:`Completed`
        (`self.K2_DestroyActor`)))))

(event `self.Projectile.OnComponentBeginOverlap`
  (params (OverlappedComponent :type "PrimitiveComponent Object Reference") (OtherActor :type "Actor Object Reference") (OtherComp :type "PrimitiveComponent Object Reference") (OtherBodyIndex :type Integer) (bFromSweep :type Boolean) (SweepResult :type "HitResult Structure (by ref)"))
  (bind _asbp_multi_monster_parent (cast `/Game/BluePrints/BP_Parents/BP_MultiMonster_Parent` OtherActor))
  (`/Engine/EditorBlueprintResources/StandardMacros.DoOnce` false
    (:`Completed`
      (`GameplayStatics.ApplyDamage` _asbp_multi_monster_parent (`self.Damage`) null self)
      (`self.K2_DestroyActor`)
      (`GameplayStatics.SpawnEmitterAtLocation` "/Game/StarterContent/Particles/P_Explosion.P_Explosion" (`self.K2_GetActorLocation`) (struct) (0.25 0.25 0.25)))))

(fn `UserConstructionScript`)