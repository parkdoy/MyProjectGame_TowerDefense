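; Tower-defense parent tower that tracks BP_MultiMonster_Parent actors inside its range sphere and fires at a randomly chosen one.
; Gated per-frame Delay loops, used instead of Tick, smoothly turn the cannon toward the target or back to rest when none remains.
; Once aim is within tolerance, a Timeline sized to the refire delay paces projectile spawns and muzzle effects.
; Clicking the tower toggles its range decal and prints its stats.
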(event `FireProjectile`
  ;[1 1 1] FireAtTarget
  (`/Engine/EditorBlueprintResources/StandardMacros.IsValid` (`self.CurrentTarget`)
    (:`Is Valid`
      (`|SpawnActorFromClass` "/Game/BluePrints/BP_Parents/BP_Projectile_parent.BP_Projectile_parent_C" (`KismetMathLibrary.MakeTransform` (.location (`SceneComponent.K2_GetComponentToWorld` (`self.CannonMesh`))) (.rotation (`SceneComponent.K2_GetComponentToWorld` (`self.CannonMesh`)))) "Undefined" "OverrideRootScale" null null)
      (`GameplayStatics.SpawnEmitterAtLocation` "/Game/FXVarietyPack/Particles/P_ky_shotShockwave.P_ky_shotShockwave" (`SceneComponent.K2_GetComponentLocation` (`self.Arrow`)) (`self.TagetAimRotator`) (0.75 0.75 0.75)))
    (:`Is Not Valid`
      (`self.StopFire`))))

(event `ContinueFire`
  ;[1 1 1] FireAtTarget
  (if (`self.CanShoot`)
    (if (== (`TimelineComponent.GetPlaybackPosition` (`self.TowerRefire`)) 0.0) :!label _label
      (`self.FireProjectile`)
      (`Timeline|TowerRefire` :!label _label_2
        (:`Finished`
          (`self.ResetFireTimeline`)
          (`self.ContinueFire`))))))

(event `ContinueAim`
  (bind _returnvalue (`KismetMathLibrary.FindLookAtRotation` (- (`self.K2_GetActorLocation` (`self.CurrentTarget`)) (`self.MonsterTargetLoc`)) (`KismetMathLibrary.InverseTransformDirection` (`self.GetTransform`) (- (`self.MonsterTargetLoc`) (`SceneComponent.K2_GetComponentLocation` (`self.CannonMesh`))))))
  (bind _returnvalue_2 (`KismetMathLibrary.RInterpTo` (`SceneComponent.RelativeRotation` (`self.CannonMesh`)) _returnvalue (`GameplayStatics.GetWorldDeltaSeconds`) (`self.TowerAimSpeed`)))
  ;[1 1 1] Aim Monster
  (`/Engine/EditorBlueprintResources/StandardMacros.IsValid` (`self.CurrentTarget`)
    (:`Is Valid`
      (`/Engine/EditorBlueprintResources/StandardMacros.Gate` true :!label _label_3
        (:`Exit`
          (`/Engine/EditorBlueprintResources/StandardMacros.IsValid` (`self.CurrentTarget`)
            (:`Is Valid`
              ;;[1 1 1] 몬스터 위치값 가져옴
              (set `self.MonsterTargetLoc` (`self.K2_GetActorLocation` (`self.CurrentTarget`)))
              (set `self.TagetAimRotator` _returnvalue)
              (`SceneComponent.K2_SetRelativeRotation` (`self.CannonMesh`) _returnvalue_2 false false)
              (if (== _returnvalue_2 (`self.TagetAimRotator`) :`ErrorTolerance` 10.0)
                (`|ExecutionSequence`
                  (:`then_0`
                    (`/Engine/EditorBlueprintResources/StandardMacros.DoOnce` false :!label _label_4
                      (:`Completed`
                        (set `self.CanShoot` true)
                        (`self.StartFire`))))
                  (:`then_1`
                    (`KismetSystemLibrary.Delay` (`GameplayStatics.GetWorldDeltaSeconds`))
                    (`self.ContinueAim`)))
                (else
                  (`self.StopFire`)
                  (`KismetSystemLibrary.Delay` (`GameplayStatics.GetWorldDeltaSeconds`))
                  (`self.ContinueAim`))))
            (:`Is Not Valid`
              (`self.CancelAim`)
              (`self.BeginReset`)
              (`self.StopFire`))))))
    (:`Is Not Valid`
      (`self.CancelAim`)
      (`self.BeginReset`))))

(event `BeginAim`
  ;[1 1 1] Aim Monster
  (`|ExecutionSequence`
    (:`then_0`
      (goto _label_3 :!via `Open`))
    (:`then_1`
      (goto _label_3))))

(event `StartFire`
  ;[1 1 1] FireAtTarget
  (`TimelineComponent.SetTimelineLength` (`self.TowerRefire`) (`self.RefireDelay`))
  (goto _label))

(event `ResetFireTrigger`
  ;[1 1 1] Aim Monster
  (goto _label_4 :!via `Reset`))

(event `CancelAim`
  ;[1 1 1] Aim Monster
  (goto _label_3 :!via `Close`))

(event `ResetFireTimeline`
  ;[1 1 1] FireAtTarget
  (`|ExecutionSequence`
    (:`then_0`
      (goto _label_2 :!via `Stop`))
    (:`then_1`
      (goto _label_2 :!via `SetNewTime`))))

(event `StopFire`
  ;[1 1 1] FireAtTarget
  (set `self.CanShoot` false)
  (`self.ResetFireTrigger`))

(event `self.ReceiveBeginPlay`
  ;[1 1 1] 감지범위설정
  (`SphereComponent.SetSphereRadius` (`self.AttackRange`) (`self.AttackRangeValue`) true)
  ;[1 1 1] Decal 영역표시
  (`SceneComponent.SetWorldScale3D` (`self.ShowRange`) (`KismetMathLibrary.Conv_DoubleToVector` (`SphereComponent.SphereRadius` (`self.AttackRange`))))
  ;[1 1 1] 범위 내에 있으면 즉시 조준..더 이상 범위 밖에 나갔다 들어와야할 필요 없음
  (`KismetSystemLibrary.Delay` (`GameplayStatics.GetWorldDeltaSeconds`))
  (for _array_element (`PrimitiveComponent.GetOverlappingActors` (`self.AttackRange`) "/Game/BluePrints/BP_Parents/BP_MultiMonster_Parent.BP_MultiMonster_Parent_C")
    (bind _asbp_multi_monster_parent (cast `/Game/BluePrints/BP_Parents/BP_MultiMonster_Parent` _array_element))
    (`KismetArrayLibrary.Array_Add` (`self.MultiMonsterTarget`) _asbp_multi_monster_parent))
  (`self.SelectTarget`))

(event `self.TowerBodyMesh.OnClicked`
  (params (TouchedComponent :type "PrimitiveComponent Object Reference") (ButtonPressed :type "Key Structure"))
  ;[1 1 1] 클릭했을때 공격범위가 나타나도록
  (bind _isa (`/Engine/EditorBlueprintResources/StandardMacros.FlipFlop` :!label _label_5)
    (:`A`
      _)
    (:`B`
      _))
  (`SceneComponent.SetVisibility` (`self.ShowRange`) _isa false)
  (`KismetSystemLibrary.PrintString` (`KismetStringLibrary.Concat_StrStr` "발사 속도 : " (`KismetStringLibrary.Conv_DoubleToString` (`self.RefireDelay`)) "공격범위 : " (`KismetStringLibrary.Conv_DoubleToString` (`self.AttackRangeValue`)) "건설비용 : " (`KismetStringLibrary.Conv_IntToString` (`self.TowerCost`))) true true (struct :`R` 0.28425 :`G` 1.0 :`B` 0.504008 :`A` 1.0)))

(event `SelectTarget`
  (bind _multimonstertarget (`self.MultiMonsterTarget`))
  ;[1 1 1] Select Target
  (if (`KismetArrayLibrary.Array_IsValidIndex` _multimonstertarget)
    (set `self.CurrentTarget` (`|GetArrayItem` _multimonstertarget (`KismetMathLibrary.RandomIntegerInRange` 0 (`KismetArrayLibrary.Array_LastIndex` _multimonstertarget))))
    ;;[1 1 1] 공격범위 체크
    (`self.BeginAim`)
    (else
      (`self.BeginReset`))))

(event `self.CannonMesh.OnClicked`
  (params (TouchedComponent :type "PrimitiveComponent Object Reference") (ButtonPressed :type "Key Structure"))
  ;[1 1 1] 클릭했을때 공격범위가 나타나도록
  (goto _label_5))

(event `ContinueReset`
  (bind _returnvalue (`KismetMathLibrary.RInterpTo` (`SceneComponent.RelativeRotation` (`self.CannonMesh`)) (struct) (`GameplayStatics.GetWorldDeltaSeconds`) 5.0))
  ;[1 1 1] Aim Reset
  (`/Engine/EditorBlueprintResources/StandardMacros.Gate` true :!label _label_6
    (:`Exit`
      (`/Engine/EditorBlueprintResources/StandardMacros.IsValid` (`self.CurrentTarget`)
        (:`Is Valid`
          (`self.CancelReset` :!label _label_7))
        (:`Is Not Valid`
          (if (== _returnvalue (struct))
            (goto _label_7)
            (else
              (`SceneComponent.K2_SetRelativeRotation` (`self.CannonMesh`) _returnvalue false false)
              (`KismetSystemLibrary.Delay` (`GameplayStatics.GetWorldDeltaSeconds`))
              (`self.ContinueReset`))))))))

(event `BeginReset`
  ;[1 1 1] Aim Reset
  (`|ExecutionSequence`
    (:`then_0`
      (goto _label_6 :!via `Open`))
    (:`then_1`
      (goto _label_6))))

(event `self.AttackRange.OnComponentBeginOverlap`
  (params (OverlappedComponent :type "PrimitiveComponent Object Reference") (OtherActor :type "Actor Object Reference") (OtherComp :type "PrimitiveComponent Object Reference") (OtherBodyIndex :type Integer) (bFromSweep :type Boolean) (SweepResult :type "HitResult Structure (by ref)"))
  ;[1 1 1] Overlap탐지
  (bind _asbp_multi_monster_parent (cast `/Game/BluePrints/BP_Parents/BP_MultiMonster_Parent` OtherActor))
  (`KismetArrayLibrary.Array_Add` (`self.MultiMonsterTarget`) _asbp_multi_monster_parent)
  (`/Engine/EditorBlueprintResources/StandardMacros.IsValid` (`self.CurrentTarget`)
    (:`Is Not Valid`
      (`self.SelectTarget`))))

(event `CancelReset`
  ;[1 1 1] Aim Reset
  (goto _label_6 :!via `Close`))

(event `self.AttackRange.OnComponentEndOverlap`
  (params (OverlappedComponent :type "PrimitiveComponent Object Reference") (OtherActor :type "Actor Object Reference") (OtherComp :type "PrimitiveComponent Object Reference") (OtherBodyIndex :type Integer))
  ;[1 1 1] Overlap탐지
  (bind _asbp_multi_monster_parent (cast `/Game/BluePrints/BP_Parents/BP_MultiMonster_Parent` OtherActor))
  (if (`KismetArrayLibrary.Array_Contains` (`self.MultiMonsterTarget`) _asbp_multi_monster_parent)
    (`KismetArrayLibrary.Array_RemoveItem` (`self.MultiMonsterTarget`) _asbp_multi_monster_parent)
    (if (== _asbp_multi_monster_parent (`self.CurrentTarget`))
      (set `self.CurrentTarget` null)
      (`self.SelectTarget`))))

(fn `UserConstructionScript`)