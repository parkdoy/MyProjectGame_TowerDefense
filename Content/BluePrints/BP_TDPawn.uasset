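; BP_TDPawn is a top-down camera pawn with keyboard panning, mouse-wheel spring-arm zoom and a Space key reset to a fixed location.
; Each Tick, MouseCursorMove calls four directional functions that edge-scroll the root by cursor viewport position.
; Left and up scrolling ramps within an edge band, while right and down triggers only at the very edge.
; Tick also snaps a decal to the surface under the cursor, oriented by impact normal.
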(event `InputAxis|MoveForward`
  (params (AxisValue :type "Float (single-precision)"))
  ;[1 1 1] 키보드 움직임 입력
  (`self.K2_AddActorLocalOffset` (`KismetMathLibrary.MakeVector` (* AxisValue (`self.MoveCamSpeed`)))))

(event `InputAxis|MoveRight`
  (params (AxisValue :type "Float (single-precision)"))
  ;[1 1 1] 키보드 움직임 입력
  (`self.K2_AddActorLocalOffset` (`KismetMathLibrary.MakeVector` 0.0 (* AxisValue (`self.MoveCamSpeed`)))))

(event `Key|MouseScrollUp`
  (params (Key :type "Key Structure"))
  (bind _springarm (`self.SpringArm`))
  ;[1 1 1] 카메라 줌인&아웃
  (:`Pressed`
    (set `SpringArmComponent.TargetArmLength` (- (`SpringArmComponent.TargetArmLength` _springarm) 100.0) _springarm)))

(event `Key|MouseScrollDown`
  (params (Key :type "Key Structure"))
  (bind _springarm (`self.SpringArm`))
  ;[1 1 1] 카메라 줌인&아웃
  (:`Pressed`
    (set `SpringArmComponent.TargetArmLength` (+ (`SpringArmComponent.TargetArmLength` _springarm) 100.0) _springarm)))

(event `Key|SpaceBar`
  (params (Key :type "Key Structure"))
  (:`Pressed`
    (`self.K2_SetActorLocation` (100.0 0.0 300.0))))

(event `self.ReceiveTick`
  (params (DeltaSeconds :type "Float (single-precision)"))
  (bind (_bblockinghit _binitialoverlap _time _distance _location _impactpoint _normal _impactnormal) (`GameplayStatics.BreakHitResult` (`PlayerController.GetHitResultUnderCursorByChannel` (`GameplayStatics.GetPlayerController` 0) "TraceTypeQuery1" true)))
  ;[1 1 1] 마우스로 이동
  (`self.MouseCursorMove`)
  (`SceneComponent.K2_SetWorldLocationAndRotation` (`self.Decal`) _location (`KismetMathLibrary.MakeRotationFromAxes` _impactnormal) false false))

(fn `MouseCursorMove`
  (`self.MoveCursorLeft`)
  (`self.MoveCursorRight`)
  (`self.MoveCursorUp`)
  (`self.MoveCursorDown`))

(fn `MoveCursorDown`
  (bind (_returnvalue_x _returnvalue_y) (`KismetMathLibrary.BreakVector2D` (`WidgetLayoutLibrary.GetViewportSize`)))
  (bind _returnvalue (`WidgetLayoutLibrary.GetMousePositionOnViewport`))
  (`SceneComponent.K2_AddRelativeLocation` (`self.DefaultSceneRoot`) (* (0.0 5.0 0.0) (`KismetMathLibrary.FClamp` (`KismetMathLibrary.NormalizeToRange` (`.Y` (`KismetMathLibrary.BreakVector2D` _returnvalue)) (* _returnvalue_y 1.0) _returnvalue_y))) false false))

(fn `MoveCursorLeft`
  (bind _returnvalue_x (`KismetMathLibrary.BreakVector2D` (`WidgetLayoutLibrary.GetViewportSize`)))
  (bind _returnvalue (`WidgetLayoutLibrary.GetMousePositionOnViewport`))
  (`SceneComponent.K2_AddRelativeLocation` (`self.DefaultSceneRoot`) (* (-5.0 0.0 0.0) (- 1.0 (`KismetMathLibrary.FClamp` (`KismetMathLibrary.NormalizeToRange` (`KismetMathLibrary.BreakVector2D` _returnvalue) 0.0 (* _returnvalue_x 0.2))))) false false))

(fn `MoveCursorRight`
  (bind _returnvalue_x (`KismetMathLibrary.BreakVector2D` (`WidgetLayoutLibrary.GetViewportSize`)))
  (bind _returnvalue (`WidgetLayoutLibrary.GetMousePositionOnViewport`))
  (`SceneComponent.K2_AddRelativeLocation` (`self.DefaultSceneRoot`) (* (5.0 0.0 0.0) (`KismetMathLibrary.FClamp` (`KismetMathLibrary.NormalizeToRange` (`KismetMathLibrary.BreakVector2D` _returnvalue) (* _returnvalue_x 1.0) _returnvalue_x))) false false))

(fn `MoveCursorUp`
  (bind (_returnvalue_x _returnvalue_y) (`KismetMathLibrary.BreakVector2D` (`WidgetLayoutLibrary.GetViewportSize`)))
  (bind _returnvalue (`WidgetLayoutLibrary.GetMousePositionOnViewport`))
  (`SceneComponent.K2_AddRelativeLocation` (`self.DefaultSceneRoot`) (* (0.0 -5.0 0.0) (- 1.0 (`KismetMathLibrary.FClamp` (`KismetMathLibrary.NormalizeToRange` (`.Y` (`KismetMathLibrary.BreakVector2D` _returnvalue)) 0.0 (* _returnvalue_y 0.2))))) false false))

(fn `UserConstructionScript`)