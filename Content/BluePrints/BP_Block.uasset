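; BP_Block is a clickable block that serves as a tower build spot, with cursor feedback shown by swapping its Cube material.
; Clicking when CanSpawnTower is true removes existing top-level UMG_TowerBuild widgets, then opens a new one with its EmptyBlock set to this block.
; Otherwise, clicking shows a disabled material.
; Hover applies a highlight material, while releasing or leaving restores the default.
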(event `self.Cube.OnClicked`
  (params (TouchedComponent :type "PrimitiveComponent Object Reference") (ButtonPressed :type "Key Structure"))
  (if (`self.CanSpawnTower`)
    (`PrimitiveComponent.SetMaterial` (`self.Cube`) 0 "/Game/MyMaterial/M_BlockClick.M_BlockClick")
    (bind _foundwidgets (`WidgetBlueprintLibrary.GetAllWidgetsOfClass` "/Game/UMG/UMG_TowerBuild.UMG_TowerBuild_C"))
    (for _array_element _foundwidgets
      (`Widget.RemoveFromParent` _array_element))
    (bind _returnvalue (`|CreateWidget` "/Game/UMG/UMG_TowerBuild.UMG_TowerBuild_C"))
    (`UserWidget.AddToViewport` _returnvalue 0)
    (set `/Game/UMG/UMG_TowerBuild.EmptyBlock` self _returnvalue)
    (else
      (`PrimitiveComponent.SetMaterial` (`self.Cube`) 0 "/Game/MyMaterial/M_BlockDisable.M_BlockDisable"))))

(event `self.Cube.OnReleased`
  (params (TouchedComponent :type "PrimitiveComponent Object Reference") (ButtonReleased :type "Key Structure"))
  (`PrimitiveComponent.SetMaterial` (`self.Cube`) 0 "/Game/MyMaterial/M_BlockColorDefault.M_BlockColorDefault" :!label _label))

(event `self.Cube.OnEndCursorOver`
  (params (TouchedComponent :type "PrimitiveComponent Object Reference"))
  (goto _label))

(event `self.Cube.OnBeginCursorOver`
  (params (TouchedComponent :type "PrimitiveComponent Object Reference"))
  (`PrimitiveComponent.SetMaterial` (`self.Cube`) 0 "/Game/MyMaterial/M_BlockOverlap.M_BlockOverlap"))

(fn `UserConstructionScript`)